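; Level piece blueprint for procedural generation that spreads the layout by spawning generator actors on its top, right, down and left sides.
; After a short BeginPlay delay, it increments a shared counter (Yolo) in RandomGameMode and branches only while that stays under 25.
; Overlap events flag occupied sides, so each spawn point either spawns its directional generator or skips it, then is destroyed.
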(event `self.ReceiveBeginPlay`
  (bind _spawn_left (`self.Spawn_Left`))
  (bind _spawn_top (`self.Spawn_Top`))
  (bind _spawn_right (`self.Spawn_Right`))
  (bind _spawn_down (`self.Spawn_Down`))
  (`KismetSystemLibrary.Delay` 0.3)
  (bind _asrandom_game_mode (cast `/Game/Levels/LevelGenerator/levelShapes/BPs/RandomGameMode` (`GameplayStatics.GetGameMode`)))
  (bind _yolo (`/Game/Levels/LevelGenerator/levelShapes/BPs/RandomGameMode.yolo` _asrandom_game_mode))
  (set `/Game/Levels/LevelGenerator/levelShapes/BPs/RandomGameMode.yolo` (+ _yolo 1) _asrandom_game_mode)
  (if (< _yolo 25)
    (`|ExecutionSequence`
      (:`then_0`
        (if (`self.OverlapTop`)
          (`ActorComponent.K2_DestroyComponent` _spawn_top :!label _label)
          (elif (`KismetSystemLibrary.IsValid` _spawn_top)
            (`|SpawnActorFromClass` "/Game/Levels/LevelGenerator/levelShapes/BPs/Generator_Top.Generator_Top_C" (`self.GetLocation` _spawn_top) "Undefined" "OverrideRootScale" null null)
            (goto _label))))
      (:`then_1`
        (if (`self.OverlapRight`)
          (`ActorComponent.K2_DestroyComponent` _spawn_right :!label _label_2)
          (elif (`KismetSystemLibrary.IsValid` _spawn_right)
            (`|SpawnActorFromClass` "/Game/Levels/LevelGenerator/levelShapes/BPs/Generator_Right.Generator_Right_C" (`self.GetLocation` _spawn_right) "Undefined" "OverrideRootScale" null null)
            (goto _label_2))))
      (:`then_2`
        (if (`self.OverlapDown`)
          (`ActorComponent.K2_DestroyComponent` _spawn_down :!label _label_3)
          (elif (`KismetSystemLibrary.IsValid` _spawn_down)
            (`|SpawnActorFromClass` "/Game/Levels/LevelGenerator/levelShapes/BPs/Generator_Down.Generator_Down_C" (`self.GetLocation` _spawn_down) "Undefined" "OverrideRootScale" null null)
            (goto _label_3))))
      (:`then_3`
        (if (`self.OverlapLeft`)
          (`ActorComponent.K2_DestroyComponent` _spawn_left :!label _label_4)
          (elif (`KismetSystemLibrary.IsValid` _spawn_left)
            (`|SpawnActorFromClass` "/Game/Levels/LevelGenerator/levelShapes/BPs/Generator_Left.Generator_Left_C" (`self.GetLocation` _spawn_left) "Undefined" "OverrideRootScale" null null)
            (goto _label_4)))))))

(event `self.Spawn_Top.OnComponentBeginOverlap`
  (params (OverlappedComponent :type "PrimitiveComponent Object Reference") (OtherActor :type "Actor Object Reference") (OtherComp :type "PrimitiveComponent Object Reference") (OtherBodyIndex :type Integer) (bFromSweep :type Boolean) (SweepResult :type "HitResult Structure (by ref)"))
  (set `self.OverlapTop` true)
  (`KismetSystemLibrary.PrintString` "Hello" :!label _label_5))

(event `self.Spawn_Right.OnComponentBeginOverlap`
  (params (OverlappedComponent :type "PrimitiveComponent Object Reference") (OtherActor :type "Actor Object Reference") (OtherComp :type "PrimitiveComponent Object Reference") (OtherBodyIndex :type Integer) (bFromSweep :type Boolean) (SweepResult :type "HitResult Structure (by ref)"))
  (set `self.OverlapRight` true)
  (goto _label_5))

(event `self.Spawn_Down.OnComponentBeginOverlap`
  (params (OverlappedComponent :type "PrimitiveComponent Object Reference") (OtherActor :type "Actor Object Reference") (OtherComp :type "PrimitiveComponent Object Reference") (OtherBodyIndex :type Integer) (bFromSweep :type Boolean) (SweepResult :type "HitResult Structure (by ref)"))
  (set `self.OverlapDown` true)
  (goto _label_5))

(event `self.Spawn_Left.OnComponentBeginOverlap`
  (params (OverlappedComponent :type "PrimitiveComponent Object Reference") (OtherActor :type "Actor Object Reference") (OtherComp :type "PrimitiveComponent Object Reference") (OtherBodyIndex :type Integer) (bFromSweep :type Boolean) (SweepResult :type "HitResult Structure (by ref)"))
  (set `self.OverlapLeft` true)
  (goto _label_5))

(fn `UserConstructionScript`)