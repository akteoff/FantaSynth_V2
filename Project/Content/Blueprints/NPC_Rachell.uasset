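; NPC_Rachell is an NPC actor that shows an interaction prompt and penalizes the player if it is destroyed.
; An Interaction overlap volume sets the Protag_BP player's text render to the PressE text and shows it on entry, then hides it on exit.
; When the actor is destroyed, it sets the player character's HP to zero and flags it as hit.
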(event `self.Interaction.OnComponentBeginOverlap`
  (params (OverlappedComponent :type "PrimitiveComponent Object Reference") (OtherActor :type "Actor Object Reference") (OtherComp :type "PrimitiveComponent Object Reference") (OtherBodyIndex :type Integer) (bFromSweep :type Boolean) (SweepResult :type "HitResult Structure (by ref)"))
  (bind _asprotag_bp (cast `/Game/Blueprints/Protag/Protag_BP` OtherActor))
  (bind _textrender (`/Game/Blueprints/Protag/Protag_BP.TextRender` _asprotag_bp))
  (`TextRenderComponent.K2_SetText` _textrender (`self.press E`))
  (`SceneComponent.SetVisibility` _textrender true false))

(event `self.Interaction.OnComponentEndOverlap`
  (params (OverlappedComponent :type "PrimitiveComponent Object Reference") (OtherActor :type "Actor Object Reference") (OtherComp :type "PrimitiveComponent Object Reference") (OtherBodyIndex :type Integer))
  (bind _asprotag_bp (cast `/Game/Blueprints/Protag/Protag_BP` OtherActor))
  (`SceneComponent.SetVisibility` (`/Game/Blueprints/Protag/Protag_BP.TextRender` _asprotag_bp) false false))

(event `self.ReceiveDestroyed`
  (bind _asprotag_bp (cast `/Game/Blueprints/Protag/Protag_BP` (`GameplayStatics.GetPlayerCharacter` 0)))
  (set `/Game/Blueprints/Protag/Protag_BP.Protag_HP` 0.0 _asprotag_bp)
  (set `/Game/Blueprints/Protag/Protag_BP.ProtagHit` true _asprotag_bp))

(fn `UserConstructionScript`)