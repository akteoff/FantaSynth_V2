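; Collectible page pickup that shows a random sprite from its set and reveals page information when the protagonist overlaps its sphere.
; LosuLosu selects either a random entry or the fixed WhichOneThen index into the game instance's page arrays.
; The chosen title and text become active and are removed from the pool, a page widget opens, and Simulation drops slightly.
; An empty pool in random mode only prints a message, and the actor then destroys itself.
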(event `self.ReceiveBeginPlay`
  (bind _possible_sprites (`self.Possible Sprites`))
  (`PaperSpriteComponent.SetSprite` (`self.PaperSprite`) (`|GetArrayItem` _possible_sprites (`KismetMathLibrary.RandomInteger` (`KismetArrayLibrary.Array_Length` _possible_sprites)))))

(event `self.Sphere.OnComponentBeginOverlap`
  (params (OverlappedComponent :type "PrimitiveComponent Object Reference") (OtherActor :type "Actor Object Reference") (OtherComp :type "PrimitiveComponent Object Reference") (OtherBodyIndex :type Integer) (bFromSweep :type Boolean) (SweepResult :type "HitResult Structure (by ref)"))
  (bind _randompageindex (`self.RandomPageIndex`))
  (cast `/Game/Blueprints/Protag/Protag_BP` OtherActor)
  (bind _asfanta_synth_game_instance (cast `/Game/Blueprints/FantaSynth_GameInstance` (`GameplayStatics.GetGameInstance`)))
  (if (`self.LosuLosu`)
    (bind _pages_information (`/Game/Blueprints/FantaSynth_GameInstance.Pages_Information` _asfanta_synth_game_instance))
    (bind _returnvalue (`KismetArrayLibrary.Array_Length` _pages_information))
    (if (> _returnvalue 0)
      (set `self.RandomPageIndex` (`KismetMathLibrary.RandomInteger` _returnvalue))
      (set `/Game/Blueprints/FantaSynth_GameInstance.Active_Info` (`|GetArrayItem` _pages_information _randompageindex) _asfanta_synth_game_instance :!label _label)
      (bind _pages_tittle (`/Game/Blueprints/FantaSynth_GameInstance.Pages_Tittle` _asfanta_synth_game_instance))
      (set `/Game/Blueprints/FantaSynth_GameInstance.Active_Tittle` (`|GetArrayItem` _pages_tittle _randompageindex) _asfanta_synth_game_instance)
      (`KismetArrayLibrary.Array_Remove` _pages_tittle _randompageindex)
      (`KismetArrayLibrary.Array_Remove` _pages_information _randompageindex)
      (bind _returnvalue_2 (`|CreateWidget` "/Game/Blueprints/Znajdzki/PageWidget.PageWidget_C"))
      (`UserWidget.AddToViewport` _returnvalue_2 0)
      (set `/Game/Blueprints/FantaSynth_GameInstance.Simulation%` (- (`/Game/Blueprints/FantaSynth_GameInstance.Simulation%` _asfanta_synth_game_instance) 0.1) _asfanta_synth_game_instance)
      (else
        (`KismetSystemLibrary.PrintString` "I already know that" true true (struct :`R` 0.025693 :`G` 1.0 :`A` 1.0))))
    (else
      (set `self.RandomPageIndex` (`self.WhichOne, then?`))
      (goto _label)))
  (`self.K2_DestroyActor`))

(fn `UserConstructionScript`)