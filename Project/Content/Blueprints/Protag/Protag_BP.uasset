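; Player character for a top-down Paper2D shooter, with axis movement and a mouse-aimed wand.
; Tick updates the walk flipbook, wand rotation, active hand and attack color, and briefly slows time when ProtagHit is set.
; Left click fires from the active wand, either a single projectile or guarded bursts of randomly spread projectiles, toggled by Space.
; An overlap sphere collects InteractionInterface targets, and Interact triggers the first.
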(event `InputAxis|UpOrDown`
  (params (AxisValue :type "Float (single-precision)"))
  ;[1 1 1] Movement
  (`self.AddMovementInput` (0.0 1.0 0.0) AxisValue))

(event `InputAxis|Left or Right`
  (params (AxisValue :type "Float (single-precision)"))
  ;[1 1 1] Movement
  (`self.AddMovementInput` (1.0 0.0 0.0) AxisValue))

(event `self.ReceiveTick`
  (params (DeltaSeconds :type "Float (single-precision)"))
  (`|ExecutionSequence`
    (:`then_0`
      (`self.WandRotate`))
    (:`then_1`
      (`self.SetProtagFlipbook`))
    (:`then_2`
      (`self.WandSpot`))
    (:`then_3`
      ;[1 1 1] changing Wand color
      (if (== (`self.SelectAttack`) 2.0)
        (`PrimitiveComponent.SetMaterial` (`self.Plane`) 0 "/Game/Sprites/Protag/WandAndProjectiles/WandCokir_blue.WandCokir_blue")
        (`PrimitiveComponent.SetMaterial` (`self.Plane1`) 0 "/Game/Sprites/Protag/WandAndProjectiles/WandCokir_blue.WandCokir_blue")
        (else
          (`PrimitiveComponent.SetMaterial` (`self.Plane`) 0 "/Game/Sprites/Protag/WandAndProjectiles/NeonProjectile_Pink.NeonProjectile_Pink")
          (`PrimitiveComponent.SetMaterial` (`self.Plane1`) 0 "/Game/Sprites/Protag/WandAndProjectiles/NeonProjectile_Pink.NeonProjectile_Pink"))))
    (:`then_4`
      ;[1 1 1] Immune after hit
      (if (`self.ProtagHit`)
        (`GameplayStatics.SetGlobalTimeDilation` 0.3)
        (`KismetSystemLibrary.Delay` 0.2)
        (`GameplayStatics.SetGlobalTimeDilation` 1.0)
        (set `self.ProtagHit` false)))))

(event `Key|LeftMouseButton`
  (params (Key :type "Key Structure"))
  ;[1 1 1] Atak
  (:`Pressed`
    (if (`self.WandInRightHand`)
      (`SceneComponent.SetVisibility` (`self.Plane`) true false)
      (`KismetSystemLibrary.Delay` 0.1)
      (`SceneComponent.SetVisibility` (`self.Plane`) false false)
      (else
        (`SceneComponent.SetVisibility` (`self.Plane1`) true false)
        (`KismetSystemLibrary.Delay` 0.1)
        (`SceneComponent.SetVisibility` (`self.Plane1`) false false)))
    (if (== (`self.SelectAttack`) 1.0)
      (`self.Attack1`)
      (elif (== (`self.SelectAttack`) 2.0)
        (if (not (`self.Attack2Activated`))
          (set `self.Attack2Activated` true)
          (`self.Attack2`)
          (`KismetSystemLibrary.Delay` 0.1)
          (`self.Attack2`)
          (`KismetSystemLibrary.Delay` 0.1)
          (`self.Attack2`)
          (`KismetSystemLibrary.Delay` 0.1)
          (`self.Attack2`)
          (`KismetSystemLibrary.Delay` 0.3)
          (set `self.Attack2Activated` false))
        (else
          (`KismetSystemLibrary.PrintString` "WrongSelectAttack"))))))

(event `Key|SpaceBar`
  (params (Key :type "Key Structure"))
  ;[1 1 1] Wybór Ataku
  (:`Pressed`
    (`GameplayStatics.SpawnSound2D` "/Game/Imports/Sounds/intarface_hover.intarface_hover" 1.0 1.0 0.0 null)
    (if (== (`self.SelectAttack`) 1.0)
      (set `self.SelectAttack` 2.0)
      (elif (== (`self.SelectAttack`) 2.0)
        (set `self.SelectAttack` 1.0)))))

(event `self.InteractionSphere.OnComponentBeginOverlap`
  (params (OverlappedComponent :type "PrimitiveComponent Object Reference") (OtherActor :type "Actor Object Reference") (OtherComp :type "PrimitiveComponent Object Reference") (OtherBodyIndex :type Integer) (bFromSweep :type Boolean) (SweepResult :type "HitResult Structure (by ref)"))
  ;[1 1 1] Interaction
  (bind _asinteraction_interface (cast `/Game/Blueprints/InteractionInterface` OtherActor)
    (:`then`
      (`KismetArrayLibrary.Array_AddUnique` (`self.InteractablesInRange`) _asinteraction_interface))
    (:`CastFailed`
      (for _array_element (`self.GetComponentsByInterface` OtherActor "/Game/Blueprints/InteractionInterface.InteractionInterface_C")
        (`KismetArrayLibrary.Array_AddUnique` (`self.InteractablesInRange`) (cast `/Game/Blueprints/InteractionInterface` _array_element :!pure true))))))

(event `self.InteractionSphere.OnComponentEndOverlap`
  (params (OverlappedComponent :type "PrimitiveComponent Object Reference") (OtherActor :type "Actor Object Reference") (OtherComp :type "PrimitiveComponent Object Reference") (OtherBodyIndex :type Integer))
  ;[1 1 1] Interaction
  (bind _asinteraction_interface (cast `/Game/Blueprints/InteractionInterface` OtherActor)
    (:`then`
      (`KismetArrayLibrary.Array_RemoveItem` (`self.InteractablesInRange`) _asinteraction_interface))
    (:`CastFailed`
      (for _array_element (`self.GetComponentsByInterface` OtherActor "/Game/Blueprints/InteractionInterface.InteractionInterface_C")
        (`KismetArrayLibrary.Array_RemoveItem` (`self.InteractablesInRange`) (cast `/Game/Blueprints/InteractionInterface` _array_element :!pure true))))))

(event `InputAction|Interact`
  (params (Key :type "Key Structure"))
  ;[1 1 1] Interaction
  (:`Pressed`
    (if (> (`KismetArrayLibrary.Array_Length` (`self.InteractablesInRange`)) 0)
      (`/Game/Blueprints/InteractionInterface.OnInteraction` (`|GetArrayItem` (`self.InteractablesInRange`)) self)
      (`KismetSystemLibrary.PrintString` "Interaction"))))

(fn `Attack1`
  (bind _returnvalue (`|SpawnActorFromClass` "/Game/Sprites/Protag/WandAndProjectiles/WandProjectile.WandProjectile_C" (`KismetMathLibrary.MakeTransform` (`self.WandLoc`) (`KismetMathLibrary.FindLookAtRotation` (+ (* (`SceneComponent.K2_GetComponentLocation` (`self.Sprite`)) (1.0 1.0 0.0)) (0.0 0.003 0.0)) (+ (* (`.Location` (`GameplayStatics.BreakHitResult` (`PlayerController.GetHitResultUnderCursorByChannel` (`GameplayStatics.GetPlayerController` 0) "TraceTypeQuery1" true))) (1.0 1.0 0.0)) (0.0 0.003 0.0)))) "Undefined" "OverrideRootScale" null null))
  (set `self.NewWandProjectile` _returnvalue))

(fn `Attack2`
  (for _ (range 1 6)
    (`|SpawnActorFromClass` "/Game/Sprites/Protag/WandAndProjectiles/WandProjectile2.WandProjectile2_C" (`KismetMathLibrary.MakeTransform` (`self.WandLoc`) (`KismetMathLibrary.MakeRotator` (.roll (`KismetMathLibrary.FindLookAtRotation` (+ (* (`SceneComponent.K2_GetComponentLocation` (`self.Sprite`)) (1.0 1.0 0.0)) (0.0 0.003 0.0)) (+ (* (`.Location` (`GameplayStatics.BreakHitResult` (`PlayerController.GetHitResultUnderCursorByChannel` (`GameplayStatics.GetPlayerController` 0) "TraceTypeQuery1" true))) (1.0 1.0 0.0)) (0.0 0.003 0.0)))) (.pitch (`KismetMathLibrary.FindLookAtRotation` (+ (* (`SceneComponent.K2_GetComponentLocation` (`self.Sprite`)) (1.0 1.0 0.0)) (0.0 0.003 0.0)) (+ (* (`.Location` (`GameplayStatics.BreakHitResult` (`PlayerController.GetHitResultUnderCursorByChannel` (`GameplayStatics.GetPlayerController` 0) "TraceTypeQuery1" true))) (1.0 1.0 0.0)) (0.0 0.003 0.0)))) (+ (.yaw (`KismetMathLibrary.FindLookAtRotation` (+ (* (`SceneComponent.K2_GetComponentLocation` (`self.Sprite`)) (1.0 1.0 0.0)) (0.0 0.003 0.0)) (+ (* (`.Location` (`GameplayStatics.BreakHitResult` (`PlayerController.GetHitResultUnderCursorByChannel` (`GameplayStatics.GetPlayerController` 0) "TraceTypeQuery1" true))) (1.0 1.0 0.0)) (0.0 0.003 0.0)))) (`KismetMathLibrary.RandomFloatInRange` -20.0 20.0)))) "Undefined" "OverrideRootScale" null null)
    (set `self.NewWandProjectile` null)))

(fn `SetProtagFlipbook`
  (bind _lastmovedirection (`self.LastMoveDirection`))
  (if (or (!= (`self.GetInputAxisValue`) 0.0) (!= (`self.GetInputAxisValue`) 0.0))
    (set `self.LastMoveDirection` (select `bool` (> (`self.GetInputAxisValue`) 0.0) :`false` (select `bool` (< (`self.GetInputAxisValue`) 0.0) :`false` (select `bool` (> (`self.GetInputAxisValue`) 0.0) :`false` (select `bool` (< (`self.GetInputAxisValue`) 0.0) :`false` "NewEnumerator0" :`true` "NewEnumerator2" :!type "/Game/Blueprints/Protag/Walk_Direction Enum") :`true` "NewEnumerator3") :`true` "NewEnumerator0") :`true` "NewEnumerator1"))
    (`PaperFlipbookComponent.SetFlipbook` (`self.Sprite`) (select `bool` (> (`KismetMathLibrary.VSize` (`self.GetVelocity`)) 0.0) :`false` (select `/Game/Blueprints/Protag/Walk_Direction` _lastmovedirection :`NewEnumerator0` "/Game/Sprites/Protag/Idle/Idle.Idle" :`NewEnumerator1` "/Game/Sprites/Protag/Idle/Idle.Idle" :`NewEnumerator2` "/Game/Sprites/Protag/Idle/Idle.Idle" :`NewEnumerator3` "/Game/Sprites/Protag/Idle/Idle.Idle" :!type "PaperFlipbook Object Reference") :`true` (select `/Game/Blueprints/Protag/Walk_Direction` _lastmovedirection :`NewEnumerator0` "/Game/Sprites/Protag/Run/WalkUp.WalkUp" :`NewEnumerator1` "/Game/Sprites/Protag/Run/WalkDown.WalkDown" :`NewEnumerator2` "/Game/Sprites/Protag/Run/WalkLeft.WalkLeft" :`NewEnumerator3` "/Game/Sprites/Protag/Run/WalkRight.WalkRight" :!type "PaperFlipbook Object Reference")))
    (else
      (`PaperFlipbookComponent.SetFlipbook` (`self.Sprite`) "/Game/Sprites/Protag/Idle/Idle.Idle"))))

(fn `Teleport`
  (`self.K2_TeleportTo` (0.0 0.0 0.0)))

(fn `UserConstructionScript`)

(fn `WandRotate`
  (`SceneComponent.K2_SetRelativeRotation` (`self.wand_Sprite_left`) (`KismetMathLibrary.MakeRotator` -90.0 0.0 (+ (.yaw (`KismetMathLibrary.FindLookAtRotation` (`SceneComponent.K2_GetComponentLocation` (`self.Sprite`)) (`.Location` (`GameplayStatics.BreakHitResult` (`PlayerController.GetHitResultUnderCursorByChannel` (`GameplayStatics.GetPlayerController` 0) "TraceTypeQuery1" true))))) 180.0)) false false)
  (`SceneComponent.K2_SetRelativeRotation` (`self.sprite_wand_right`) (`KismetMathLibrary.MakeRotator` -90.0 0.0 (.yaw (`KismetMathLibrary.FindLookAtRotation` (`SceneComponent.K2_GetComponentLocation` (`self.Sprite`)) (`.Location` (`GameplayStatics.BreakHitResult` (`PlayerController.GetHitResultUnderCursorByChannel` (`GameplayStatics.GetPlayerController` 0) "TraceTypeQuery1" true)))))) false false))

(fn `WandSpot`
  (if (> (.x (`.Location` (`GameplayStatics.BreakHitResult` (`PlayerController.GetHitResultUnderCursorByChannel` (`GameplayStatics.GetPlayerController` 0) "TraceTypeQuery1" true)))) (.x (`self.K2_GetActorLocation`)))
    (set `self.WandInRightHand` true)
    (set `self.WandLoc` (`SceneComponent.K2_GetComponentLocation` (`self.Plane`)))
    (`SceneComponent.SetVisibility` (`self.wand_Sprite_left`) false false)
    (`SceneComponent.SetVisibility` (`self.sprite_wand_right`) true false)
    (else
      (set `self.WandInRightHand` false)
      (set `self.WandLoc` (`SceneComponent.K2_GetComponentLocation` (`self.Plane1`)))
      (`SceneComponent.SetVisibility` (`self.sprite_wand_right`) false false)
      (`SceneComponent.SetVisibility` (`self.wand_Sprite_left`) true false))))