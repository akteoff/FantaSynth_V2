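; Trigger volume that turns nearby enemies aggressive when the player character (Protag_BP) enters it.
; On begin overlap, a sequence fetches all actors of five enemy classes: Fast, Range, HGB, BGB and Drag.
; Each actor overlapping the collision component gets its Agressive flag set to true, so only enemies inside the volume at that moment are alerted.
; Nothing in the Blueprint clears the flag.
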(event `self.ReceiveActorBeginOverlap`
  (params (OtherActor :type "Actor Object Reference"))
  (cast `/Game/Blueprints/Protag/Protag_BP` OtherActor)
  (`|ExecutionSequence`
    (:`then_0`
      (bind _outactors (`GameplayStatics.GetAllActorsOfClass` "/Game/Blueprints/Enemies/Head_Goblin/Fast_Enemy.Fast_Enemy_C"))
      (for _array_element _outactors
        (if (`PrimitiveComponent.IsOverlappingActor` (`self.CollisionComponent`) _array_element)
          (set `/Game/Blueprints/Enemies/Head_Goblin/Fast_Enemy.Agressive?` true _array_element))))
    (:`then_1`
      (bind _outactors_2 (`GameplayStatics.GetAllActorsOfClass` "/Game/Blueprints/Enemies/Bow_Goblin/Range_Enemy.Range_Enemy_C"))
      (for _array_element_2 _outactors_2
        (if (`PrimitiveComponent.IsOverlappingActor` (`self.CollisionComponent`) _array_element_2)
          (set `/Game/Blueprints/Enemies/Bow_Goblin/Range_Enemy.Agressive` true _array_element_2))))
    (:`then_2`
      (bind _outactors_3 (`GameplayStatics.GetAllActorsOfClass` "/Game/Blueprints/Enemies/Head_Goblin_Broken/HGB_Enemy.HGB_Enemy_C"))
      (for _array_element_3 _outactors_3
        (if (`PrimitiveComponent.IsOverlappingActor` (`self.CollisionComponent`) _array_element_3)
          (set `/Game/Blueprints/Enemies/Head_Goblin_Broken/HGB_Enemy.Agressive?` true _array_element_3))))
    (:`then_3`
      (bind _outactors_4 (`GameplayStatics.GetAllActorsOfClass` "/Game/Blueprints/Enemies/Bow_Goblin_Broken/BGB_Enemy.BGB_Enemy_C"))
      (for _array_element_4 _outactors_4
        (if (`PrimitiveComponent.IsOverlappingActor` (`self.CollisionComponent`) _array_element_4)
          (set `/Game/Blueprints/Enemies/Bow_Goblin_Broken/BGB_Enemy.Agressive?` true _array_element_4))))
    (:`then_4`
      (bind _outactors_5 (`GameplayStatics.GetAllActorsOfClass` "/Game/Blueprints/Enemies/Dargon/drag.drag_C"))
      (for _array_element_5 _outactors_5
        (if (`PrimitiveComponent.IsOverlappingActor` (`self.CollisionComponent`) _array_element_5)
          (set `/Game/Blueprints/Enemies/Dargon/drag.Agressive?` true _array_element_5))))))

(fn `UserConstructionScript`)